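; Player-controllable tank Blueprint that handles camera look, track-based driving and cannon fire.
; On BeginPlay it passes its turret, barrel and left and right track mesh components to setter functions.
; Camera axes yaw a gimbal and pitch the spring arm (inverted) separately.
; Separate throttle axes call MoveTracks on each track, and the fire action calls ShootCannon.
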(event `self.ReceiveBeginPlay`
  (`self.SetTurret` (`self.MeshTurret`))
  (`self.SetBarrel` (`self.MeshBarrel`))
  (`self.SetTracks` (`self.MeshLTrack`) (`self.MeshRTrack`)))

(event `InputAxis|CameraRotX`
  (params (AxisValue :type "Float (single-precision)"))
  (`SceneComponent.K2_AddLocalRotation` (`self.GimbalRotX`) (`KismetMathLibrary.MakeRotator` 0.0 0.0 AxisValue) false false))

(event `InputAxis|CameraRotY`
  (params (AxisValue :type "Float (single-precision)"))
  (`SceneComponent.K2_AddLocalRotation` (`self.SpringArm`) (`KismetMathLibrary.MakeRotator` 0.0 (* AxisValue -1.0)) false false))

(event `InputAction|Shoot_Cannon`
  (params (Key :type "Key Structure"))
  (:`Pressed`
    (`self.ShootCannon`)))

(event `InputAxis|LeftThrottle`
  (params (AxisValue :type "Float (single-precision)"))
  (`MeshTankTracks.MoveTracks` (`self.MeshLTrack`) AxisValue))

(event `InputAxis|RightThrottle`
  (params (AxisValue :type "Float (single-precision)"))
  (`MeshTankTracks.MoveTracks` (`self.MeshRTrack`) AxisValue))

(fn `UserConstructionScript`)